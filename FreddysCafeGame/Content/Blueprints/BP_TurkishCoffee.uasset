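; Turkish coffee recipe actor that defines the drink's preparation steps: Measure, Grind, Boil and Finish.
; On BeginPlay it names itself, then a Sequence spawns an ingredient actor per step at its own transform, though the last spawn shows no class.
; Each is initialized with step name, display name, mesh, view target ID and icon, then appended in order to IngredientList.
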(event EventBeginPlay
  (bind _returnvalue (Transformation|GetActorTransform))
  (bind _ingredientlist (Variables|Default|GetIngredientList))
  (Variables|Default|SetName "Turkish Coffee")
  (Utilities|FlowControl|Sequence
    (:then_0
      (bind _returnvalue_2 (Game|SpawnActorfromClass "/Game/Blueprints/BP_Ingredient.BP_Ingredient_C" _returnvalue "Undefined" "MultiplyWithRoot" 0 0))
      (Default|Initialize _returnvalue_2 "Measure" "Coffee Beans" "/Game/Assets/measuringCUP.measuringCUP" 1 "/Game/Assets/icons/icon_measure.icon_measure")
      (Utilities|Array|Add _ingredientlist _returnvalue_2))
    (:then_1
      (bind _returnvalue_3 (Game|SpawnActorfromClass "/Game/Blueprints/BP_Ingredient.BP_Ingredient_C" _returnvalue "Undefined" "MultiplyWithRoot" 0 0))
      (Default|Initialize _returnvalue_3 "Grind" "Grinder" "/Game/Assets/coffeeGrinderBODY.coffeeGrinderBODY" 1 "/Game/Assets/icons/icon_grind.icon_grind")
      (Utilities|Array|Add _ingredientlist _returnvalue_3))
    (:then_2
      (bind _returnvalue_4 (Game|SpawnActorfromClass "/Game/Blueprints/BP_Ingredient.BP_Ingredient_C" _returnvalue "Undefined" "MultiplyWithRoot" 0 0))
      (Default|Initialize _returnvalue_4 "Boil" "Ground Coffee" "/Game/EF_FirstFloor/Meshes/pot_b.pot_b" 3 "/Game/Assets/icons/icon_boil.icon_boil")
      (Utilities|Array|Add _ingredientlist _returnvalue_4))
    (:then_3
      (bind _returnvalue_5 (Game|SpawnActorfromClass "/Game/Blueprints/BP_Ingredient.BP_Ingredient_C" _returnvalue "Undefined" "MultiplyWithRoot" 0 0))
      (Default|Initialize _returnvalue_5 "Finish" "Coffee Cup" "/Game/Assets/coffeecupEMPTY.coffeecupEMPTY" 3 "/Game/Assets/icons/icon_cup.icon_cup")
      (Utilities|Array|Add _ingredientlist _returnvalue_5))))

(event Collision|EventActorBeginOverlap
  (params (OtherActor :type Actor%20Object%20Reference)))

(event EventTick
  (params (DeltaSeconds :type Float%20%28single-precision%29)))

(fn ConstructionScript)